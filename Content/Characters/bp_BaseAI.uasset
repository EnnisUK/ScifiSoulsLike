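; Base AI character that the player can lock onto and damage, handing the lock-on target to another AI when it dies.
; Lockon and EndLockon toggle its decal through ShowHideDecal.
; Damage calls TakeDamage, then ignores further hits for a short delay.
; Death removes itself from the list of all BaseAI actors, then sets the main character's HitTarget to the one nearest the player, if within range.
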(event `self.ReceiveBeginPlay`
  (set `self.m_LockedOnDecal` (`self.Decal`))
  (bind _asbp_main_character (cast `/Game/Characters/bp_MainCharacter` (`GameplayStatics.GetPlayerCharacter` 0)))
  (set `self.As Bp Main Character` _asbp_main_character))

(event `self.ReceiveTick`
  (params (DeltaSeconds :type "Float (single-precision)")))

(event `AIInterface.Lockon`
  (`self.Show_HideDecal` (`self.Decal`) true))

(event `AIInterface.EndLockon`
  (`self.Show_HideDecal` (`self.Decal`)))

(event `AIInterface.Damage`
  (params (DamageAmount :type "Float (single-precision)"))
  (if (not (`self.m_IsTakingDamage`))
    (set `self.m_IsTakingDamage` true)
    (`|ExecutionSequence`
      (:`then_0`
        (`self.TakeDamage` DamageAmount))
      (:`then_1`
        (`KismetSystemLibrary.Delay` 1.5)
        (set `self.m_IsTakingDamage` false)))))

(event `AIInterface.Death`
  (bind _outactors (`GameplayStatics.GetAllActorsOfClass` "/Script/ScifiSoulsLike.BaseAI"))
  (bind _output_get (set `self.BaseAIAllActors` _outactors))
  (bind _returnvalue (`KismetArrayLibrary.Array_RemoveItem` _output_get self))
  (if _returnvalue
    (`self.SelectNextTarget`)))

(event `SelectNextTarget`
  (bind _returnvalue (`GameplayStatics.GetPlayerCharacter` 0))
  (bind (_distance _returnvalue_2) (`GameplayStatics.FindNearestActor` (`self.K2_GetActorLocation` _returnvalue) (`self.BaseAIAllActors`)))
  (bind _asbp_main_character (cast `/Game/Characters/bp_MainCharacter` _returnvalue))
  (if (< _distance 1000.0)
    (set `MainCharacter.m_HitTarget` _returnvalue_2 _asbp_main_character)
    (else
      (`KismetSystemLibrary.PrintString` "Not Close Enough"))))

(fn `UserConstructionScript`)