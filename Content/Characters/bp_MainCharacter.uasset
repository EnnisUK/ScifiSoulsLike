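; Main character Blueprint that drives blocking, rolling and jumping through the Gameplay Ability System and equips a sword and shield on BeginPlay.
; Enhanced Input actions activate abilities by tag, and releasing block removes effects granting the IsBlocking tag.
; Falling, gated by a DoOnce that landing resets, and landing apply airborne and grounded gameplay effects, while Tick updates a grounded flag.
; Helper functions toggle the anim Blueprint's blocking state.
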(event `self.ReceiveBeginPlay`
  (`self.AddEquipment` "WeaponSocket" "/Game/BP/Equipment/BP_Sword.BP_Sword_C")
  (`self.AddEquipment` "ShieldSocket" "/Game/BP/Equipment/BP_Shield.BP_Shield_C")
  (`AbilitySystemComponent.BP_ApplyGameplayEffectToSelf` :`self` (`self.m_AbilitySystemComponent`) :`GameplayEffectClass` "/Game/BP/Abilities/Jumping/GE_IsGrounded.GE_IsGrounded_C"))

(event `EnhancedInput|/Game/ThirdPerson/Input/Actions/IA_Block`
  (params (ActionValue :type Boolean) (ElapsedSeconds :type "Float (double-precision)") (TriggeredSeconds :type "Float (double-precision)") (InputAction :type "InputAction Object Reference" :default "/Game/ThirdPerson/Input/Actions/IA_Block.IA_Block"))
  (bind _m_abilitysystemcomponent (`self.m_AbilitySystemComponent`))
  ;[1 1 1] Blocking
  (:`Triggered`
    (`AbilitySystemComponent.TryActivateAbilitiesByTag` _m_abilitysystemcomponent (`self.Blocking Tag Container`) true :!label _label))
  (:`Ongoing`
    (goto _label))
  (:`Completed`
    (`AbilitySystemComponent.RemoveActiveEffectsWithGrantedTags` _m_abilitysystemcomponent (struct :`GameplayTags` (struct :`(TagName` "Player.IsBlocking"))))))

(event `EnhancedInput|/Game/ThirdPerson/Input/Actions/IA_Roll`
  (params (ActionValue :type Boolean) (ElapsedSeconds :type "Float (double-precision)") (TriggeredSeconds :type "Float (double-precision)") (InputAction :type "InputAction Object Reference" :default "/Game/ThirdPerson/Input/Actions/IA_Roll.IA_Roll"))
  (:`Triggered`
    (`AbilitySystemComponent.TryActivateAbilitiesByTag` (`self.m_AbilitySystemComponent`) (`self.Rolling Tag Container`) true)))

(event `self.ReceiveTick`
  (params (DeltaSeconds :type "Float (single-precision)"))
  (set `self.m_IsGrounded` (not (`NavMovementComponent.IsFalling` (`self.CharacterMovement`)))))

(event `EnhancedInput|/Game/ThirdPerson/Input/Actions/IA_Jump`
  (params (ActionValue :type Boolean) (ElapsedSeconds :type "Float (double-precision)") (TriggeredSeconds :type "Float (double-precision)") (InputAction :type "InputAction Object Reference" :default "/Game/ThirdPerson/Input/Actions/IA_Jump.IA_Jump"))
  ;[1 1 1] Jumping
  (:`Started`
    (`AbilitySystemComponent.TryActivateAbilitiesByTag` (`self.m_AbilitySystemComponent`) (`self.Jump Tag Container`) true)))

(event `Falling`
  ;[1 1 1] Jumping
  (`/Engine/EditorBlueprintResources/StandardMacros.DoOnce` false :!label _label_2
    (:`Completed`
      (`AbilitySystemComponent.BP_ApplyGameplayEffectToSelf` :`self` (`self.m_AbilitySystemComponent`) :`GameplayEffectClass` "/Game/BP/Abilities/Jumping/GE_IsAirborn.GE_IsAirborn_C"))))

(event `self.OnLanded`
  (params (Hit :type "HitResult Structure (by ref)"))
  (`self.Landed`))

(event `Landed`
  ;[1 1 1] Jumping
  (`AbilitySystemComponent.BP_ApplyGameplayEffectToSelf` :`self` (`self.m_AbilitySystemComponent`) :`GameplayEffectClass` "/Game/BP/Abilities/Jumping/GE_IsGrounded.GE_IsGrounded_C")
  (goto _label_2 :!via `Reset`))

(fn `AddEquipment`
  (params (SocketName :type Name) (Equipment :type "/Game/BP/Equipment/BP_Equipment Class Reference"))
  (bind _mesh (`self.Mesh`))
  (bind _returnvalue (`|SpawnActorFromClass` Equipment (`SceneComponent.GetSocketTransform` _mesh SocketName "RTS_World") "Undefined" "MultiplyWithRoot" null null))
  (`self.K2_AttachToComponent` _returnvalue _mesh SocketName "SnapToTarget" "SnapToTarget" "SnapToTarget" true))

(fn `Blocking`
  (bind _asmain_char_anim_bp (cast `/Game/Animations/MainCharacter/MainChar_AnimBP` (`SkeletalMeshComponent.GetAnimInstance` (`self.Mesh`))))
  (set `/Game/Animations/MainCharacter/MainChar_AnimBP.IsBlocking` true _asmain_char_anim_bp))

(fn `StopBlocking`
  (bind _asmain_char_anim_bp (cast `/Game/Animations/MainCharacter/MainChar_AnimBP` (`SkeletalMeshComponent.GetAnimInstance` (`self.Mesh`))))
  (set `/Game/Animations/MainCharacter/MainChar_AnimBP.IsBlocking` false _asmain_char_anim_bp))

(fn `UserConstructionScript`
  (`SceneComponent.K2_AttachToComponent` (`self.m_WeaponChildClass`) (`self.Mesh`) "MeleeWeaponSocket" "SnapToTarget" "SnapToTarget" "SnapToTarget" true))