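; GA_Blocking is a gameplay ability that makes the main character block.
; On activation it commits, applies GE_IsBlocking to the owner and calls Blocking on bp_MainCharacter.
; A WaitGameplayTagRemove task ends the ability when the Player.IsBlocking tag is removed.
; Ending calls StopBlocking on the character and ends the stored wait task.
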(event `self.K2_ActivateAbility`
  (`self.K2_CommitAbility`)
  (`self.BP_ApplyGameplayEffectToOwner` "/Game/BP/Abilities/Blocking/GE_IsBlocking.GE_IsBlocking_C")
  (bind _asbp_main_character (cast `/Game/Characters/bp_MainCharacter` (`.OwnerActor` (break `GameplayAbilityActorInfo` (`self.GetActorInfo`)))))
  (`/Game/Characters/bp_MainCharacter.Blocking` _asbp_main_character)
  (bind _asynctaskproxy (`AbilityTask_WaitGameplayTagRemoved.WaitGameplayTagRemove` (struct :`TagName` "Player.IsBlocking") null)
    (:`then`
      (set `self.Wait For Tag` _asynctaskproxy))
    (:`Removed`
      (`self.K2_EndAbility`))))

(event `self.K2_OnEndAbility`
  (params (bWasCancelled :type Boolean))
  (bind _wait_for_tag (`self.Wait For Tag`))
  (`/Game/Characters/bp_MainCharacter.StopBlocking` (stale `self.K2_ActivateAbility` _asbp_main_character))
  (`/Engine/EditorBlueprintResources/StandardMacros.IsValid` _wait_for_tag
    (:`Is Valid`
      (`GameplayTask.EndTask` _wait_for_tag))))